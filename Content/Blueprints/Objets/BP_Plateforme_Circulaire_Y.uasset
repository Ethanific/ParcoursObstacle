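; Moving platform actor that spins and shuttles back and forth between MinY and MaxY limits.
; Tick offsets its location by Direction and Vitesse scaled by delta time, without sweep, flipping Direction past a limit and teleporting Y back onto it.
; The lower-bound test compares the X position to MinY.Y, while the upper test uses Y.
; The construction script copies Rotations into the RotatingMovement component's rate.
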(event EventBeginPlay)

(event Collision|EventActorBeginOverlap
  (params (OtherActor :type Actor%20Object%20Reference)))

(event EventTick
  (params (DeltaSeconds :type Float%20%28single-precision%29))
  (bind _returnvalue (Transformation|GetActorRotation))
  (bind _returnvalue_2 (Transformation|GetActorLocation))
  (bind _returnvalue_3 (Transformation|GetActorLocation))
  (bind _maxy (Variables|Components|GetMaxY))
  (bind _miny (Variables|Components|GetMinY))
  (bind _returnvalue_4 (> (.y _returnvalue_2) (.y _maxy)))
  (bind _returnvalue_5 (< (.x _returnvalue_2) (.y _miny)))
  (Transformation|SetActorLocation (+ (* DeltaSeconds (Variables|Components|GetVitesse) (Variables|Components|GetDirection)) (Transformation|GetActorLocation)) false false)
  (if (or _returnvalue_5 _returnvalue_4)
    (Variables|Components|SetDirection (* (Variables|Components|GetDirection) -1))
    ;[1 1 1] Met la valeur de la position au max-min possible au cas ou il est sortie
    (if _returnvalue_5
      (bind _output_get (Variables|Components|SetTPMin (Math|Vector|MakeVector (.x _returnvalue_3) (.y _miny) (.z _returnvalue_3))))
      (Transformation|Teleport _output_get _returnvalue)
      (elif _returnvalue_4
        (bind _output_get_2 (Variables|Components|SetTPMax (Math|Vector|MakeVector (.x _returnvalue_3) (.y _maxy) (.z _returnvalue_3))))
        (Transformation|Teleport _output_get_2 _returnvalue)))))

(fn ConstructionScript
  (Variables|/Script/Engine.RotatingMovementComponent|SetRotationRate (Variables|Components|GetRotatingMovement) (Variables|Components|GetRotations)))