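; BP_Plateforme_Circulaire_Z is a moving platform that travels back and forth between two Z limits while rotating.
; Each Tick it offsets its location by Direction, scaled by Vitesse and delta time, without sweeping.
; It reverses Direction whenever its height is outside the Z components of MinZ and MaxZ, with no clamping.
; The construction script feeds the Rotations variable into a RotatingMovement component to set the spin.
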(event EventBeginPlay)

(event Collision|EventActorBeginOverlap
  (params (OtherActor :type Actor%20Object%20Reference)))

(event EventTick
  (params (DeltaSeconds :type Float%20%28single-precision%29))
  (bind _returnvalue (Transformation|GetActorLocation))
  (Transformation|SetActorLocation (+ (* DeltaSeconds (Variables|Components|GetVitesse) (Variables|Components|GetDirection)) (Transformation|GetActorLocation)) false false)
  (if (or (< (.z _returnvalue) (.z (Variables|Components|GetMinZ))) (> (.z _returnvalue) (.z (Variables|Components|GetMaxZ))))
    (Variables|Components|SetDirection (* (Variables|Components|GetDirection) -1))))

(fn ConstructionScript
  (Variables|/Script/Engine.RotatingMovementComponent|SetRotationRate (Variables|Components|GetRotatingMovement) (Variables|Components|GetRotations)))